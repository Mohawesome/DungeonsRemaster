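; Base actor for a damage-over-time effect that shows a particle while the effect lasts and then destroys itself.
; BeginPlay turns the particle on through the Multi_PlayParticle event and calls StartDOT, which on authority sets a one-shot timer derived from the damage tick count.
; When the timer fires, it turns the particle off and destroys the actor after a short delay; no damage is applied in this graph.
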(event `self.ReceiveBeginPlay`
  (`self.Multi_PlayParticle` true)
  (`self.StartDOT`))

(event `StartDOT`
  (`/Engine/EditorBlueprintResources/ActorMacros.Switch Has Authority`
    (:`Authority`
      (`KismetSystemLibrary.K2_SetTimerDelegate` (delegate `DeactivateParticle`) (`KismetMathLibrary.Conv_IntToDouble` (+ (`self.DamageTickAmount`) 1))))))

(event `DeactivateParticle`
  (`self.Multi_PlayParticle` false)
  (`KismetSystemLibrary.Delay` 1.0)
  (`self.K2_DestroyActor`))

(event `Multi_PlayParticle`
  (params (OnOff :type Boolean))
  (bind _particlesystem (`self.ParticleSystem`))
  (if OnOff
    (`ActorComponent.Activate` _particlesystem false)
    (else
      (`ActorComponent.Deactivate` _particlesystem))))

(fn `UserConstructionScript`)