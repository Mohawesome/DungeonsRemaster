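; Player controller for the dungeon game that creates the local player UI, drives pawn movement and manages lives.
; Movement axes move the cached pawn along control-rotation forward and right vectors unless the stunned flag, set through MovementFrozen, is active.
; Lives go up or down through events; respawn spawns and possesses a new pawn above the given location while lives remain, otherwise prints Game Over.
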(event `self.ReceiveBeginPlay`
  (set `self.PlayerPawn` (`self.K2_GetPawn`))
  (`KismetSystemLibrary.Delay` 0.2)
  (if (`self.IsLocalPlayerController`)
    (bind _returnvalue (`|CreateWidget` "/Game/Main/UI/PlayerUI.PlayerUI_C"))
    (bind _output_get (set `self.PlayerUI` _returnvalue))
    (`UserWidget.AddToViewport` _output_get 0)))

(event `InputAxis|MoveForward`
  (params (AxisValue :type "Float (single-precision)"))
  (bind _playerpawn (`self.PlayerPawn`))
  (`self.PlayerPawn`
    (:`then`
      (if (not (`self.PlayerStunned`))
        (`Pawn.AddMovementInput` _playerpawn (`KismetMathLibrary.GetForwardVector` (`Pawn.GetControlRotation` _playerpawn)) AxisValue false)))
    (:`else`)))

(event `/Game/Main/Interfaces/INT_PlayerController.MovementFrozen`
  (params (State :type Boolean))
  ;[1 1 1] Interfaces
  (set `self.PlayerStunned` State))

(event `/Game/Main/Interfaces/INT_PlayerController.IncreaseLives`
  ;[1 1 1] Interfaces
  (set `self.PlayerLives` (+ (`self.PlayerLives`) 1)))

(event `InputAxis|MoveRight`
  (params (AxisValue :type "Float (single-precision)"))
  (bind _playerpawn (`self.PlayerPawn`))
  (`self.PlayerPawn`
    (:`then`
      (if (not (`self.PlayerStunned`))
        (`Pawn.AddMovementInput` _playerpawn (`KismetMathLibrary.GetRightVector` (`Pawn.GetControlRotation` _playerpawn)) AxisValue false)))
    (:`else`)))

(event `/Game/Main/Interfaces/INT_PlayerController.DecreaseLives`
  ;[1 1 1] Interfaces
  (set `self.PlayerLives` (- (`self.PlayerLives`) 1)))

(event `/Game/Main/Interfaces/INT_PlayerController.PlayerRespawn`
  (params (SpawnedLocation :type "Vector Structure") (PlayerClass :type "/Game/Main/BP_PlayerBase Class Reference"))
  (if (> (`self.PlayerLives`) 0)
    (bind _returnvalue (`|SpawnActorFromClass` PlayerClass (`KismetMathLibrary.MakeTransform` (+ SpawnedLocation (0.0 0.0 150.0))) "AlwaysSpawn" "OverrideRootScale" null null))
    (`self.Possess` _returnvalue)
    (set `self.PlayerStunned` false)
    (set `self.PlayerPawn` (`self.K2_GetPawn`))
    (else
      (`KismetSystemLibrary.PrintString` "PC_DungeonsController: Game Over"))))

(fn `UserConstructionScript`)