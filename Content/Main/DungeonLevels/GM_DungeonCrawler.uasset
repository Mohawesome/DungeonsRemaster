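; Game mode for the dungeon crawler that handles player login and character class selection.
; On login it caches player starts, records the controller, then messages the host to pick a class or sends other clients the character availability array.
; A selection marks a free slot as taken (true) and returns its class, which the player controller receives for first spawn at the first player start.
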(event `self.ReceiveBeginPlay`)

(event `self.K2_PostLogin`
  (params (NewPlayer :type "PlayerController Object Reference"))
  (bind _outactors (`GameplayStatics.GetAllActorsOfClass` "/Script/Engine.PlayerStart"))
  (set `self.StartingSpawns` _outactors)
  (`KismetArrayLibrary.Array_AddUnique` (`self.ConnectedPlayers`) NewPlayer)
  (if (== NewPlayer (`GameplayStatics.GetPlayerController` 0))
    (message `/Game/Main/Interfaces/INT_PlayerController.GetClass` NewPlayer)
    (else
      (message `/Game/Main/Interfaces/INT_PlayerController.InitializeClient` NewPlayer (`self.AvailableCharacters`)))))

(event `self.GetSelectedClass`
  (params (Class :type Integer) (PC :type "/Game/Main/DungeonLevels/PC_DungeonController Object Reference"))
  (bind _character (`self.UpdateCharacters` Class))
  (message `/Game/Main/Interfaces/INT_PlayerController.PlayerFirstSpawn` PC (`self.K2_GetActorLocation` (`|GetArrayItem` (`self.StartingSpawns`))) _character))

(fn `UpdateCharacters`
  (params (SelectedCharacter :type Integer))
  (returns (Character :type "/Game/Main/BP_PlayerBase Class Reference"))
  (if (not (== (`|GetArrayItem` (`self.AvailableCharacters`) SelectedCharacter) true))
    (`KismetArrayLibrary.Array_Set` (`self.AvailableCharacters`) SelectedCharacter true)
    (return (`|GetArrayItem` (`self.Classes`) SelectedCharacter))))

(fn `UserConstructionScript`)