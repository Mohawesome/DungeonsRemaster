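; Base player Blueprint for a multiplayer game, handling health, death, potions and vendor interaction, with empty attack, ability and upgrade-info hooks for child classes.
; Input is gated on death and attack state, then routed to Server events.
; Damage can trigger a delayed respawn through the controller, which decrements lives before the actor is destroyed.
; UI, currency and movement freezing go through controller messages, while Health vendors open a purchase widget.
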(event `Server_PrimaryAttack`
  ;[1 1 1] Attack Overrides
)

(event `Server_AbilityOne`
  ;[1 1 1] Attack Overrides
)

(event `Server_AbilityTwo`
  ;[1 1 1] Attack Overrides
)

(event `Server_AbilityThree`
  ;[1 1 1] Attack Overrides
)

(event `self.ReceiveAnyDamage`
  (params (Damage :type "Float (single-precision)") (DamageType :type "DamageType Object Reference") (InstigatedBy :type "Controller Object Reference") (DamageCauser :type "Actor Object Reference"))
  (bind ((`MaxHealth_4_00A8D9224198A3E374966BBE8F69A519` _maxhealth) (`MaxMana_8_F7F62CAA4668283E08A414A1013EBD4D` _maxmana)) (break `/Game/Main/S_Stats` (`self.Stats`)))
  ;[1 1 1] Damage Event
  (if (not (`self.IsImmune`))
    (bind _structout (setmembers `/Game/Main/S_Stats` :`StructRef` (`self.Stats`) :`CurrentHealth` (- (`.CurrentHealth_2_289734A046C2CAB728B1DBA3B206683F` (break `/Game/Main/S_Stats` (`self.Stats`))) Damage)))
    (`self.Client_UpdateHealthUI` (`.CurrentHealth_2_289734A046C2CAB728B1DBA3B206683F` (break `/Game/Main/S_Stats` _structout)))
    (`self.Multi_VoiceSounds` (`self.VoicePain`) (`self.K2_GetActorLocation`))
    (if (<= (`.CurrentHealth_2_289734A046C2CAB728B1DBA3B206683F` (break `/Game/Main/S_Stats` (`self.Stats`))) 0.0)
      (`self.Server_KillPlayer`)
      (`self.Client_UpdateHealthUI` _maxhealth)
      (`self.Client_UpdateManaUI` _maxmana))))

(event `Server_KillPlayer`
  ;[1 1 1] Player Death
  (if (not (`self.IsDead`))
    (set `self.IsDead` true)
    (`self.Multi_PlayerDead`)
    (message `/Game/Main/Interfaces/INT_PlayerController.MovementFrozen` (`self.ControllerRef`) true)
    (`self.Multi_VoiceSounds` (`self.VoiceDeath`) (`self.K2_GetActorLocation`))
    (`KismetSystemLibrary.Delay` 5.0)
    (`self.Server_RespawnPlayer`)))

(event `Server_RespawnPlayer`
  (bind _controllerref (`self.ControllerRef`))
  (bind _controllerref_2 (`self.ControllerRef`))
  (bind (_currenthealth _maxhealth _currentmana _maxmana) (break `/Game/Main/S_Stats` (`self.Stats`)))
  ;[1 1 1] RespawnSystem
  (message `/Game/Main/Interfaces/INT_PlayerController.DecreaseLives` _controllerref_2)
  (message `/Game/Main/Interfaces/INT_PlayerController.PlayerRespawn` _controllerref_2 (`self.f_GetSpawnedLocation`) (`self.PlayerClass`))
  (`KismetSystemLibrary.Delay` 0.2)
  (`self.K2_DestroyActor`)
  (message `/Game/Main/Interfaces/INT_PlayerController.UpdateHealthUI` _controllerref _maxhealth)
  (message `/Game/Main/Interfaces/INT_PlayerController.UpdateManaUI` _controllerref _maxmana)
  (message `/Game/Main/Interfaces/INT_PlayerController.UpdatePotionUI` _controllerref true))

(event `UpdatePlayerMovement`
  (params (State :type Boolean))
  (if State
    (message `/Game/Main/Interfaces/INT_PlayerController.MovementFrozen` (`self.ControllerRef`) true)
    (elif (not (`self.IsDead`))
      (message `/Game/Main/Interfaces/INT_PlayerController.MovementFrozen` (`self.ControllerRef`) false))))

(event `InputAction|PrimaryAttack`
  (params (Key :type "Key Structure"))
  ;[1 1 1] Input Abilities
  (:`Pressed`
    (if (not (`self.IsDead`))
      (if (not (`self.CurrentlyAttacking`))
        (`self.Server_PrimaryAttack`)))))

(event `InputAction|AbilityOne`
  (params (Key :type "Key Structure"))
  ;[1 1 1] Input Abilities
  (:`Pressed`
    (if (not (`self.IsDead`))
      (if (not (`self.CurrentlyAttacking`))
        (`self.Server_AbilityOne`)))))

(event `InputAction|AbilityTwo`
  (params (Key :type "Key Structure"))
  ;[1 1 1] Input Abilities
  (:`Pressed`
    (if (not (`self.IsDead`))
      (if (not (`self.CurrentlyAttacking`))
        (`self.Server_AbilityTwo`)))))

(event `InputAction|AbilityThree`
  (params (Key :type "Key Structure"))
  ;[1 1 1] Input Abilities
  (:`Pressed`
    (if (not (`self.IsDead`))
      (if (not (`self.CurrentlyAttacking`))
        (`self.Server_AbilityThree`)))))

(event `InputAction|UsePotion`
  (params (Key :type "Key Structure"))
  ;[1 1 1] Input Abilities
  (:`Pressed`
    (`self.Server_UsePotion`)))

(event `Server_UsePotion`
  (bind _stats (`self.Stats`))
  ;[1 1 1] Input Abilities
  (if (`self.HasPotion`)
    (if (not (`self.IsDead`))
      (setmembers `/Game/Main/S_Stats` :`StructRef` _stats :`CurrentHealth` (`.MaxHealth_4_00A8D9224198A3E374966BBE8F69A519` (break `/Game/Main/S_Stats` _stats)))
      (set `self.HasPotion` false)
      (`self.Client_UpdateHealthUI` (`.CurrentHealth_2_289734A046C2CAB728B1DBA3B206683F` (break `/Game/Main/S_Stats` (`self.Stats`))))
      (`self.Client_UpdatePotionUI` false))))

(event `/Game/Main/Interfaces/INT_PlayerCharacter.AddPotion`
  (set `self.HasPotion` true)
  (`self.Client_UpdatePotionUI` true))

(event `/Game/Main/Interfaces/INT_PlayerCharacter.AddCurrency`
  (params (CurrencyToAdd :type Integer))
  (message `/Game/Main/Interfaces/INT_PlayerController.UpdateCurrency` (`self.ControllerRef`) CurrencyToAdd))

(event `Client_UpdateHealthUI`
  (params (CurrentHealth :type "Float (double-precision)"))
  ;[1 1 1] UpdatePlayerUI
  (message `/Game/Main/Interfaces/INT_PlayerController.UpdateHealthUI` (`self.ControllerRef`) CurrentHealth))

(event `Client_UpdateManaUI`
  (params (CurrentMana :type "Float (double-precision)"))
  ;[1 1 1] UpdatePlayerUI
  (message `/Game/Main/Interfaces/INT_PlayerController.UpdateManaUI` (`self.ControllerRef`) CurrentMana))

(event `/Game/Main/Interfaces/INT_PlayerCharacter.CloseWidgets`
  (bind _returnvalue (`GameplayStatics.GetPlayerController` 0))
  (`WidgetBlueprintLibrary.SetInputMode_GameOnly` _returnvalue)
  (set `PlayerController.bShowMouseCursor` false _returnvalue))

(event `Client_UpdatePotionUI`
  (params (Show :type Boolean))
  ;[1 1 1] UpdatePlayerUI
  (message `/Game/Main/Interfaces/INT_PlayerController.UpdatePotionUI` (`self.ControllerRef`) Show))

(event `/Game/Main/Interfaces/INT_PlayerCharacter.UpdateVendorDescription`
  (params (Description :type Text))
  (bind _vendorwidget (`self.VendorWidget`)
    (:`then`
      (`/Game/Main/Vendor/W_VendorWidget.UpdateDescription` _vendorwidget Description))
    (:`else`)))

(event `/Game/Main/Interfaces/INT_PlayerCharacter.SetInteractable`
  (params (State :type Boolean) (Interactable :type "Actor Object Reference"))
  (if State
    (set `self.Interactable` Interactable)
    (else
      (set `self.Interactable` null))))

(event `InputAction|Interact`
  (params (Key :type "Key Structure"))
  (:`Pressed`
    (bind _interactable (`self.Interactable`)
      (:`then`
        (bind _interacttype (message `/Game/Main/Interfaces/INT_Interact.GetInteractType` _interactable))
        (switch `/Game/Main/E_Interactable` _interacttype
          (:`NewEnumerator0`
            (`self.f_Vendors` (`self.Interactable`)))))
      (:`else`))))

(fn `CheckForPotion`
  (returns (HasPotion :type Boolean))
  (return (`self.HasPotion`)))

(fn `f_GetHealthPool`
  (returns (Name :type Text) (Cost :type Integer) (Description :type Text))
  ;[1 1 1] Override in child class
  (return "" 0 ""))

(fn `f_GetManaPool`
  (returns (Name :type Text) (Cost :type Integer) (Description :type Text))
  ;[1 1 1] Override in child class
  (return "" 0 ""))

(fn `f_UpdateMana`
  (params (ManaCost :type "Float (double-precision)"))
  (returns (CurrentMana :type "Float (double-precision)"))
  (bind _stats (`self.Stats`))
  (bind _structout (setmembers `/Game/Main/S_Stats` :`StructRef` _stats :`CurrentMana` (- (`.CurrentMana_6_44C47FCE44764120021447B34BA1EA3C` (break `/Game/Main/S_Stats` _stats)) ManaCost)))
  (return (`.CurrentMana_6_44C47FCE44764120021447B34BA1EA3C` (break `/Game/Main/S_Stats` _structout))))

(fn `f_Vendors`
  (params (Object :type "Actor Object Reference"))
  (bind (_name _cost _description) (`self.f_GetHealthPool`))
  (bind (_name_2 _cost_2 _description_2) (`self.f_GetManaPool`))
  (bind _returnvalue (`GameplayStatics.GetPlayerController` 0))
  (bind _vendor (message `/Game/Main/Interfaces/INT_Vendor.GetVendorType` Object))
  (switch `/Game/Main/Vendor/E_VendorType` _vendor
    (:`NewEnumerator0`
      (bind _returnvalue_2 (`|CreateWidget` "/Game/Main/Vendor/W_VendorWidget.W_VendorWidget_C" (`GameplayStatics.GetPlayerController` 0)))
      (bind _output_get (set `self.VendorWidget` _returnvalue_2))
      (`UserWidget.AddToViewport` _output_get 0)
      (`WidgetBlueprintLibrary.SetInputMode_UIOnlyEx` _returnvalue (`self.VendorWidget`))
      (set `PlayerController.bShowMouseCursor` true _returnvalue)
      (bind _vendoritems (message `/Game/Main/Interfaces/INT_Vendor.GetVendorItems` (`self.Interactable`)))
      (for (_ _array_index) _vendoritems
        (switch `int` _array_index
          (:`0`
            (bind _savedstats (message `/Game/Main/Interfaces/INT_PlayerController.GetSavedStats` (`self.GetController`)))
            (bind ((`Currency_11_0202D5CF4EA0E44030B1DDA8E57333CB` _currency)) (break `/Game/Main/S_Stats` _savedstats))
            (`/Game/Main/Vendor/W_VendorWidget.PopulateVendorItems` (`self.VendorWidget`) (`GameplayStatics.GetPlayerController` 0) _name _cost (>= _currency _cost) _description _currency))
          (:`1`
            (bind _savedstats_2 (message `/Game/Main/Interfaces/INT_PlayerController.GetSavedStats` (`self.GetController`)))
            (bind ((`Currency_11_0202D5CF4EA0E44030B1DDA8E57333CB` _currency_2)) (break `/Game/Main/S_Stats` _savedstats_2))
            (`/Game/Main/Vendor/W_VendorWidget.PopulateVendorItems` (`self.VendorWidget`) (`GameplayStatics.GetPlayerController` 0) _name_2 _cost_2 (>= _currency_2 _cost_2) _description_2 _currency_2)))))))

(fn `GetPlayerStats`
  (returns (PlayerStats :type "/Game/Main/S_Stats Structure"))
  (return (`self.Stats`)))

(fn `IsPlayerImmune`
  (returns (State :type Boolean))
  (return (`self.IsImmune`)))

(fn `PlayerDeathState`
  (returns (State :type Boolean))
  (return (`self.IsDead`)))

(fn `UserConstructionScript`)