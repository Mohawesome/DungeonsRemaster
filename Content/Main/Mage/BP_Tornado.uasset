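; Mage tornado actor that travels forward from its spawn point, damaging enemies it touches.
; A timeline lerps its location to a fixed distance ahead without sweeping, relying on capsule overlaps for hits.
; On authority, overlapping living actors tagged Enemy take damage credited to the instigator and receive a fire damage-over-time message.
; The hit list clears after each overlap, so re-entering enemies can be hit again.
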(event `self.ReceiveBeginPlay`
  (set `self.SpawnedLocation` (`self.K2_GetActorLocation`))
  (set `self.Destination` (+ (`self.SpawnedLocation`) (* (`self.GetActorForwardVector`) 1000.0)))
  (bind (_direction _alpha) (`Timeline|TornadoMovement` :!via `PlayFromStart`)
    (:`Update`
      (`self.K2_SetActorLocation` (`KismetMathLibrary.VLerp` (`self.SpawnedLocation`) (`self.Destination`) _alpha)))))

(event `self.Capsule.OnComponentBeginOverlap`
  (params (OverlappedComponent :type "PrimitiveComponent Object Reference") (OtherActor :type "Actor Object Reference") (OtherComp :type "PrimitiveComponent Object Reference") (OtherBodyIndex :type Integer) (bFromSweep :type Boolean) (SweepResult :type "HitResult Structure (by ref)"))
  (bind _hitenemies (`self.HitEnemies`))
  (`/Engine/EditorBlueprintResources/ActorMacros.Switch Has Authority`
    (:`Authority`
      (if (`self.ActorHasTag` OtherActor "Enemy")
        (bind _dead (message `/Game/Main/Interfaces/INT_EnemyBase.AIDeathCheck` OtherActor))
        (if (not _dead)
          (`KismetArrayLibrary.Array_AddUnique` _hitenemies OtherActor)
          (for _array_element _hitenemies
            (`GameplayStatics.ApplyDamage` _array_element (`self.Damage`) null (`self.GetInstigator`) "/Script/Engine.DamageType")
            (message `/Game/Main/Interfaces/INT_EnemyBase.DamageOverTime` _array_element (`self.DamageOverTime`) (`self.TickAmount`) "/Game/Main/Mage/BP_DOT_Fire.BP_DOT_Fire_C"))
          (`KismetArrayLibrary.Array_Clear` (`self.HitEnemies`)))))))

(fn `UserConstructionScript`)