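; Player controller for the main menu that creates and shows the menu widget and handles gamepad confirmation.
; On BeginPlay it disables input, adds W_MainMenu to the viewport, then after a short delay focuses it in Game and UI mode with a visible cursor and re-enables input.
; The gamepad bottom face button switches on the selected index, with only the first entry wired, to trigger New Game.
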(event `self.ReceiveBeginPlay`
  (`self.DisableInput` null)
  (bind _returnvalue (`|CreateWidget` "/Game/Main/MainMenu/W_MainMenu.W_MainMenu_C"))
  (bind _output_get (set `self.MainMenu` _returnvalue))
  (`UserWidget.AddToViewport` _output_get 0)
  (`KismetSystemLibrary.Delay` 3.0)
  (`WidgetBlueprintLibrary.SetInputMode_GameAndUIEx` self (`self.MainMenu`))
  (set `self.bShowMouseCursor` true)
  (`self.EnableInput` null))

(event `Key|Gamepad_FaceButton_Bottom`
  (params (Key :type "Key Structure"))
  (:`Pressed`
    (switch `int` (`self.CurrentlySelectedIndex`)
      (:`0`
        (`/Game/Main/MainMenu/W_MainMenu.Gamepad_NewGameBtn(On Clicked)` (`self.MainMenu`))))))

(fn `UserConstructionScript`)