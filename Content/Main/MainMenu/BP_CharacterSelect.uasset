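; BP_CharacterSelect is a main menu character display for character selection, with a skeletal mesh and a spotlight.
; SpotlightSwitch shows or hides the spotlight, and CharacterSelected plays the Paladin or Mage selection montage on the mesh according to the character passed in.
; StopMontage halts slot animation on the mesh's anim instance with a short blend-out.
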(event `SpotlightSwitch`
  (params (Switch :type Boolean))
  (bind _spotlight (`self.SpotLight`))
  (if Switch
    (`SceneComponent.SetVisibility` _spotlight true false)
    (else
      (`SceneComponent.SetVisibility` _spotlight false false))))

(event `CharacterSelected`
  (params (Character :type "/Game/Main/MainMenu/E_CharacterSelect Enum" :default "NewEnumerator0"))
  (bind _skeletalmesh (`self.SkeletalMesh`))
  (switch `/Game/Main/MainMenu/E_CharacterSelect` Character
    (:`NewEnumerator0`
      (`|PlayMontage` _skeletalmesh "/Game/Main/MainMenu/Paladin_Selected.Paladin_Selected"))
    (:`NewEnumerator1`
      (`|PlayMontage` _skeletalmesh "/Game/Main/MainMenu/Mage_Selected.Mage_Selected"))))

(event `StopMontage`
  (`AnimInstance.StopSlotAnimation` (`SkeletalMeshComponent.GetAnimInstance` (`self.SkeletalMesh`)) 0.25 "None"))

(fn `UserConstructionScript`)