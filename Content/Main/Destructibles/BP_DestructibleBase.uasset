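; Base destructible actor that shatters as soon as it begins play and drops a random item.
; BeginPlay sets the RepNotify variable Break, whose OnRep applies heavy damage and an impulse to the DestructibleComponent at the actor's location.
; The component's fracture event, on authority only, spawns one of the first two SpawnedItem classes at the actor's transform, ignoring collisions.
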(event `self.ReceiveBeginPlay`
  (set `self.Break` true))

(event `self.DestructibleComponent.OnComponentFracture`
  (params (HitPoint :type "Vector Structure (by ref)") (HitDirection :type "Vector Structure (by ref)"))
  (`/Engine/EditorBlueprintResources/ActorMacros.Switch Has Authority`
    (:`Authority`
      (`|SpawnActorFromClass` (`|GetArrayItem` (`self.SpawnedItem`) (`KismetMathLibrary.RandomIntegerInRange` 0 1)) (`self.GetTransform`) "AlwaysSpawn" "OverrideRootScale" null null))))

(fn `OnRep_Break`
  (bind _returnvalue (`self.K2_GetActorLocation`))
  (if (`self.Break`)
    (`DestructibleComponent.ApplyDamage` (`self.DestructibleComponent`) 2000.0 _returnvalue _returnvalue (`self.ImpulseStrength`))))

(fn `UserConstructionScript`)