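; BP_DestructibleObject is a replicated breakable prop that shatters when something overlaps its Box.
; On authority, the overlap sets Destroy and calls a server item-drop event.
; OnRep_Destroy swaps the static mesh for the Destructible, disables Box collision and applies heavy damage with a random impulse.
; The drop event only rolls a 40% chance, as the random item spawn and delayed actor destruction are disconnected.
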(event `self.Box.OnComponentBeginOverlap`
  (params (OverlappedComponent :type "PrimitiveComponent Object Reference") (OtherActor :type "Actor Object Reference") (OtherComp :type "PrimitiveComponent Object Reference") (OtherBodyIndex :type Integer) (bFromSweep :type Boolean) (SweepResult :type "HitResult Structure (by ref)"))
  (`/Engine/EditorBlueprintResources/ActorMacros.Switch Has Authority`
    (:`Authority`
      (set `self.Destroy` true)
      (`self.Server_SpawnItemDrop`))))

(event `Server_SpawnItemDrop`
  (if (`/Game/Main/BP_MacroLibrary.PercentChance` 40.0)
    _))

(fn `OnRep_Destroy`
  (bind _returnvalue (`self.K2_GetActorLocation`))
  (`SceneComponent.SetVisibility` (`self.StaticMesh`) false false)
  (`SceneComponent.SetVisibility` (`self.Destructible`) true false)
  (`PrimitiveComponent.SetCollisionEnabled` (`self.Box`) "NoCollision")
  (`DestructibleComponent.ApplyDamage` (`self.Destructible`) 5000.0 _returnvalue _returnvalue (`KismetMathLibrary.RandomFloatInRange` 800.0 1500.0)))

(fn `UserConstructionScript`)