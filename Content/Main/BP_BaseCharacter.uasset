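; BP_BaseCharacter is a base character that provides shared montage and sound events for attacks, hits and stuns.
; On BeginPlay it caches the controller, spawn location and anim instance after a short delay; AISpawnedLocation can re-record the spawn point.
; Multi_-prefixed events play montages and sounds, with the attack sound triggered by the montage's notify.
; Helper functions return a random attack section and the stored spawn location.
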(event `self.ReceiveBeginPlay`
  (`KismetSystemLibrary.Delay` 0.5)
  (set `self.ControllerRef` (`self.GetController`))
  (set `self.SpawnLocation` (`self.K2_GetActorLocation`))
  (set `self.AnimInstance` (`SkeletalMeshComponent.GetAnimInstance` (`self.Mesh`))))

(event `AISpawnedLocation`
  (set `self.SpawnLocation` (`self.K2_GetActorLocation`)))

(event `Multi_PrimaryAttack`
  (params (InSkeletalMeshComponent :type "SkeletalMeshComponent Object Reference") (MontageToPlay :type "AnimMontage Object Reference") (StartingSection :type Name) (AttackSound :type "SoundBase Object Reference"))
  (`|PlayMontage` InSkeletalMeshComponent MontageToPlay 1.0 0.0 StartingSection
    (:`OnNotifyBegin`
      (`GameplayStatics.PlaySoundAtLocation` AttackSound (`self.K2_GetActorLocation`) (struct) 1.0 1.0 0.0 null null null))))

(event `Multi_PlayHitSound`
  (params (Sound :type "SoundBase Object Reference") (Location :type "Vector Structure"))
  (`GameplayStatics.PlaySoundAtLocation` Sound Location (struct) 1.0 1.0 0.0 null null null))

(event `Multi_StunnedMontage`
  (params (InSkeletalMeshComponent :type "SkeletalMeshComponent Object Reference") (MontageToPlay :type "AnimMontage Object Reference"))
  (`|PlayMontage` InSkeletalMeshComponent MontageToPlay))

(fn `f_GetMontageSection`
  (returns (Section :type Name))
  (bind _attacksections (`self.AttackSections`))
  (return (`|GetArrayItem` _attacksections (`KismetMathLibrary.RandomIntegerInRange` 0 (- (`KismetArrayLibrary.Array_Length` _attacksections) 1)))))

(fn `f_GetSpawnedLocation`
  (returns (SpawnedLocation :type "Vector Structure"))
  (return (`self.SpawnLocation`)))

(fn `UserConstructionScript`)