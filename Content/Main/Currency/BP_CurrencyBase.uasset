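; Base currency pickup that grants its currency amount to a player-tagged actor overlapping its sphere.
; The overlap is handled only with authority and passes the amount to that actor through AddCurrencyMessage.
; An Added flag blocks repeat grants, and the pickup hides itself, then destroys itself after a short delay.
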(event `self.Sphere.OnComponentBeginOverlap`
  (params (OverlappedComponent :type "PrimitiveComponent Object Reference") (OtherActor :type "Actor Object Reference") (OtherComp :type "PrimitiveComponent Object Reference") (OtherBodyIndex :type Integer) (bFromSweep :type Boolean) (SweepResult :type "HitResult Structure (by ref)"))
  (`/Engine/EditorBlueprintResources/ActorMacros.Switch Has Authority`
    (:`Authority`
      (if (`self.ActorHasTag` OtherActor "Player")
        (if (not (`self.Added`))
          (message `/Game/Main/Interfaces/INT_PlayerCharacter.AddCurrency` OtherActor (`self.CurrencyAmount`))
          (`self.UpdateAndDestroy`))))))

(event `UpdateAndDestroy`
  (set `self.Added` true)
  (`self.SetActorHiddenInGame` true)
  (`KismetSystemLibrary.Delay` 0.4)
  (`self.K2_DestroyActor`))

(fn `UserConstructionScript`)